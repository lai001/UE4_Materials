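; Test actor that plays an MP3 from the project's Assets folder and runs audio analysis on a sound submix.
; On BeginPlay it binds envelope follower and spectral analysis delegates on the submix, using loop-generated, linearly spaced frequency bands.
; Once the media opens, MediaSound is sent to that submix; a failed open prints the missing file.
; Analysis callbacks convert their float arrays to strings but leave the results unused.
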(event `self.ReceiveBeginPlay`
  (bind _returnvalue (`MediaSoundComponent.GetMediaPlayer` (`self.MediaSound`)))
  (`self.AddDelegates`)
  (add `MediaPlayer.OnMediaOpened` _returnvalue (delegate `OnMediaOpened_Event`))
  (add `MediaPlayer.OnMediaOpenFailed` _returnvalue (delegate `OnMediaOpenFailed_Event`))
  (bind _path (`self.GetAssetsFolderPath`))
  (`MediaPlayer.OpenFile` _returnvalue (`KismetStringLibrary.Concat_StrStr` _path "/8_bit_mentality.mp3")))

(event `OnMediaOpened_Event`
  (params (OpenedUrl :type String))
  (`SynthComponent.SetSubmixSend` (`self.MediaSound`) (`self.SoudMixer`) 1.0))

(event `OnMediaOpenFailed_Event`
  (params (FailedUrl :type String))
  (`KismetSystemLibrary.PrintText` (`|FormatText` "Please make ensure the file ({Url}) is exists" FailedUrl)))

(event `AddDelegates`
  (bind _soudmixer (`self.SoudMixer`))
  (`SoundSubmix.AddEnvelopeFollowerDelegate` _soudmixer (delegate `CustomEvent`))
  (`SoundSubmix.StartEnvelopeFollowing` _soudmixer)
  (bind _settings (`self.MakeBandSettings`))
  (`SoundSubmix.AddSpectralAnalysisDelegate` (`self.SoudMixer`) _settings (delegate `CustomEvent_0`) 10.0 -40.0 true false 0.1 60.0)
  (`SoundSubmix.StartSpectralAnalysis` (`self.SoudMixer`) "DefaultSize" "Linear" "Hann" 0.0 "MagnitudeSpectrum"))

(event `CustomEvent`
  (params (Envelope :type "Array of Float (single-precision) (by ref)"))
  (`self.FloatArrayToString` Envelope))

(event `CustomEvent_0`
  (params (Magnitude :type "Array of Float (single-precision) (by ref)"))
  (`self.FloatArrayToString` Magnitude))

(fn `FloatArrayToString`
  (params (Values :type "Array of Float (double-precision)"))
  (returns (Str :type String))
  (locals (OutputStr :type String))
  (for _array_element Values
    (set `local.OutputStr` (`KismetTextLibrary.Conv_TextToString` (`|FormatText` "{A} {B}" (`local.OutputStr`) _array_element))))
  (return (`local.OutputStr`)))

(fn `GetAssetsFolderPath`
  (returns (Path :type String))
  (return (`KismetStringLibrary.Concat_StrStr` (`KismetSystemLibrary.GetProjectDirectory`) "Assets")))

(fn `MakeBandSettings`
  (returns (Settings :type "Array of SoundSubmixSpectralAnalysisBandSettings Structure"))
  (locals (BandSettings :type "Array of SoundSubmixSpectralAnalysisBandSettings Structure"))
  (for _index (range 10 139)
    (`KismetArrayLibrary.Array_Add` (`local.BandSettings`) (make `SoundSubmixSpectralAnalysisBandSettings` (* _index 10.0))))
  (return (`local.BandSettings`)))

(fn `UserConstructionScript`)